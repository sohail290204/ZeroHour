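; Chest actor Blueprint that plays open and close animations and can reveal hidden body meshes.
; OpenChest and CloseChest set the ChestOpen and ChestClose flags and play the matching non-looping animation on the chest skeletal mesh.
; BeginPlay hides two additional skeletal meshes, and UnhideBody shows one of them according to whether BodyCount is 1 or 2.
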(event `Open Chest`
  (set `self.ChestOpen` true)
  (set `self.ChestClose` false)
  (`SkeletalMeshComponent.PlayAnimation` (`self.SkeletalMesh`) "/Game/Assets/Chest/Chest1/Chest_Anim_Armature_A_Open.Chest_Anim_Armature_A_Open" false))

(event `Close Chest`
  (set `self.ChestOpen` false)
  (set `self.ChestClose` true)
  (`SkeletalMeshComponent.PlayAnimation` (`self.SkeletalMesh`) "/Game/Assets/Chest/Chest1/Chest_Anim_Armature_A_Close.Chest_Anim_Armature_A_Close" false))

(event `self.ReceiveBeginPlay`
  (`SceneComponent.SetHiddenInGame` (`self.SkeletalMesh1`) true false)
  (`SceneComponent.SetHiddenInGame` (`self.SkeletalMesh2`) true false))

(event `UnhideBody`
  (switch `int` (`self.BodyCount`)
    (:`1`
      (`SceneComponent.SetHiddenInGame` (`self.SkeletalMesh1`) false false))
    (:`2`
      (`SceneComponent.SetHiddenInGame` (`self.SkeletalMesh2`) false false))))

(fn `UserConstructionScript`)