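; Door bomb actor that explodes once when a Bp_MainDoorWithBomb stops overlapping its Box component.
; It spawns a scaled-up explosion emitter at its location and runs a multi sphere trace on the Visibility channel around itself.
; Any BP_ThirdPersonCharacter hit loses health directly and runs its CheckDEAD check.
; The bomb destroys itself from inside the hit loop, so only when the trace returns hits.
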(event `self.Box.OnComponentEndOverlap`
  (params (OverlappedComponent :type "PrimitiveComponent Object Reference") (OtherActor :type "Actor Object Reference") (OtherComp :type "PrimitiveComponent Object Reference") (OtherBodyIndex :type Integer))
  (bind _returnvalue (`self.K2_GetActorLocation`))
  (cast `/Game/Assets/Door/MainDoor1/Bp_MainDoorWithBomb` OtherActor)
  (`/Engine/EditorBlueprintResources/StandardMacros.DoOnce` false
    (:`Completed`
      (`GameplayStatics.SpawnEmitterAtLocation` "/Game/StarterContent/Particles/P_Explosion.P_Explosion" (`self.K2_GetActorLocation`) (struct) (10.0 10.0 10.0))
      (bind _outhits (`KismetSystemLibrary.SphereTraceMulti` _returnvalue _returnvalue 500.0 "TraceTypeQuery1"))
      (for _array_element _outhits
        (bind _asbp_third_person_character (cast `/Game/ThirdPerson/Blueprints/BP_ThirdPersonCharacter` (`.HitActor` (`GameplayStatics.BreakHitResult` _array_element)))
          (:`then`
            (set `/Game/ThirdPerson/Blueprints/BP_ThirdPersonCharacter.PlayerHealth` (- (`/Game/ThirdPerson/Blueprints/BP_ThirdPersonCharacter.PlayerHealth` _asbp_third_person_character) 100.0) _asbp_third_person_character)
            (`/Game/ThirdPerson/Blueprints/BP_ThirdPersonCharacter.CheckDEAD` _asbp_third_person_character)
            (`self.K2_DestroyActor`))
          (:`CastFailed`
            (`self.K2_DestroyActor`)))))))

(fn `UserConstructionScript`)