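; Energy drink pickup actor that adds to the player's item inventory when picked up.
; PickUpItems calls IncreaseCount, destroys the actor and returns the item's name and type.
; IncreaseCount casts the player pawn to BP_ThirdPersonCharacter and increments the entry for the item's name in its ItemCounts map.
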(event `Increase count`
  (bind _asbp_third_person_character (cast `/Game/ThirdPerson/Blueprints/BP_ThirdPersonCharacter` (`GameplayStatics.GetPlayerPawn` 0)))
  (bind _itemcounts (`/Game/ThirdPerson/Blueprints/BP_ThirdPersonCharacter.ItemCounts` _asbp_third_person_character))
  (`BlueprintMapLibrary.Map_Add` _itemcounts (`self.Name`) (+ (`BlueprintMapLibrary.Map_Find` _itemcounts (`self.Name`)) 1)))

(fn `PickUpItems`
  (returns (ItemName :type String) (ItemType :type "/Game/Inventory/Enum_InventoryTypes Enum"))
  (`self.Increase count`)
  (`self.K2_DestroyActor`)
  (return (`self.Name`) (`self.ItemType`)))

(fn `UserConstructionScript`
  (`parent.UserConstructionScript`))