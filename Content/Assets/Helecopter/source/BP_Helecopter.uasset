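; BP_Helecopter is a helicopter actor that carries the hidden player pawn for 30 seconds, then destroys itself.
; On BeginPlay it attaches the pawn to Arrow1 and snaps itself to StartLocation.
; A looping timer plays a recoil camera shake at its position, presumably to simulate vibration.
; The Timeline lerp toward EndLocation is disconnected and TimerLocation is empty, so this graph drives no flight movement.
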(event `self.ReceiveBeginPlay`
  (bind _returnvalue (`GameplayStatics.GetPlayerPawn` 0))
  (`|ExecutionSequence`
    (:`then_0`
      (`self.SetActorHiddenInGame` _returnvalue true)
      (`self.K2_AttachToComponent` _returnvalue (`self.Arrow1`) "b19" "SnapToTarget" "SnapToTarget" "SnapToTarget" false)
      (`self.K2_SetActorLocation` (`self.StartLocation`))
      (`self.TimerLocation`)
      (`KismetSystemLibrary.Delay` 30.0)
      (`self.K2_DestroyActor`))
    (:`then_1`
      (`KismetSystemLibrary.K2_SetTimerDelegate` (delegate `CustomEvent`) 0.1 true))))

(event `CustomEvent`
  (`GameplayStatics.PlayWorldCameraShake` "/Game/ThirdPerson/Blueprints/Recoil/M4_Normal_RecoilCamerShake.M4_Normal_RecoilCamerShake_C" (`self.K2_GetActorLocation`) 50.0 100.0 1.0 true))

(event `Location`)

(event `TimerLocation`)

(fn `UserConstructionScript`)