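; BP_Locker is a hiding-locker actor that the player character can get into and out of.
; OpenLocker plays the open animation and blends the player camera to the locker, then immediately calls CloseLocker, which plays the close animation.
; Pressing H starts the open animation, blends the view back to BP_ThirdPersonCharacter, calls its GetOutOfLocker and likewise calls CloseLocker with no delay.
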(event `Open Locker`
  (set `self.OpenLocker` true)
  (`SkeletalMeshComponent.PlayAnimation` (`self.SkeletalMesh`) "/Game/Assets/Locker/NewFolder/LockerOpen.LockerOpen" false)
  (`PlayerController.SetViewTargetWithBlend` (`GameplayStatics.GetPlayerController` 0) self 0.5 "VTBlend_Linear" 0.0 false)
  (`self.Close Locker`))

(event `Key|H`
  (params (Key :type "Key Structure"))
  (:`Pressed`
    (`SkeletalMeshComponent.PlayAnimation` (`self.SkeletalMesh`) "/Game/Assets/Locker/NewFolder/LockerOpen.LockerOpen" false)
    (`SkeletalMeshComponent.PlayAnimation` (`self.SkeletalMesh`) "/Game/Assets/Locker/NewFolder/LockerOpen.LockerOpen" false)
    (bind _returnvalue (`GameplayStatics.GetActorOfClass` "/Game/ThirdPerson/Blueprints/BP_ThirdPersonCharacter.BP_ThirdPersonCharacter_C"))
    (`PlayerController.SetViewTargetWithBlend` (`GameplayStatics.GetPlayerController` 0) _returnvalue 0.5 "VTBlend_Linear" 0.0 false)
    (`/Game/ThirdPerson/Blueprints/BP_ThirdPersonCharacter.GetOutOfLocker` _returnvalue)
    (`self.Close Locker`)))

(event `Close Locker`
  (set `self.OpenLocker` false)
  (`SkeletalMeshComponent.PlayAnimation` (`self.SkeletalMesh`) "/Game/Assets/Locker/NewFolder/LockerClose.LockerClose" false))

(fn `UserConstructionScript`)