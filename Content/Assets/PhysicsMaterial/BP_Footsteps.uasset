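; BP_Footsteps is an animation notify that plays surface-specific footstep sounds.
; On notify, it line-traces on Visibility from an X-offset of the owner's location, with the endpoint multiplying that position by a scaled negative up vector rather than adding it.
; The hit's physical surface selects a wood, grass, gravel or concrete sound, played at player character 0's location instead of the animated mesh owner's.
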(fn `NewFunction`)

(fn `Received_Notify`
  (params (MeshComp :type "SkeletalMeshComponent Object Reference") (Animation :type "AnimSequenceBase Object Reference") (EventReference :type "AnimNotifyEventReference Structure (by ref)"))
  (returns (ReturnValue :type Boolean))
  (bind _returnvalue (`ActorComponent.GetOwner` MeshComp))
  (bind _returnvalue_2 (`Actor.K2_GetActorLocation` (`GameplayStatics.GetPlayerCharacter` 0)))
  (bind _returnvalue_3 (+ (`Actor.K2_GetActorLocation` _returnvalue) (100.0 0.0 0.0)))
  (bind (_outhit _returnvalue_4) (`KismetSystemLibrary.LineTraceSingle` _returnvalue_3 (* _returnvalue_3 (* (`Actor.GetActorUpVector` _returnvalue) -200.0)) "TraceTypeQuery1"))
  (if _returnvalue_4
    (switch `EPhysicalSurface` (`GameplayStatics.GetSurfaceType` _outhit)
      (:`SurfaceType1`
        (`GameplayStatics.PlaySoundAtLocation` "/Game/Assets/Sounds/FootSteps/Indoor/IndoorFootSteps.IndoorFootSteps" _returnvalue_2 (struct) 1.0 1.0 0.0 null null null null))
      (:`SurfaceType2`
        (`GameplayStatics.PlaySoundAtLocation` "/Game/Assets/Sounds/FootSteps/Grass/Grass.Grass" _returnvalue_2 (struct) 1.0 1.0 0.0 null null null null))
      (:`SurfaceType3`
        (`GameplayStatics.PlaySoundAtLocation` "/Game/Assets/Sounds/FootSteps/Gravel/Gravel.Gravel" _returnvalue_2 (struct) 1.0 1.0 0.0 null null null null))
      (:`SurfaceType4`
        (`GameplayStatics.PlaySoundAtLocation` "/Game/Assets/Sounds/FootSteps/Concreate/Concrete.Concrete" _returnvalue_2 (struct) 1.0 1.0 0.0 null null null null))))
  (return false))