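; Ladder actor that lets BP_ThirdPersonCharacter climb, driven by overlap volumes that set state flags on the character.
; The main volume toggles climbing, while floor and top volumes track which end the player is at.
; Unless the player is flagged on top, the upper-side volume locks input, flags the climb end, then after a fixed delay moves the capsule to an Arrow marker.
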(event `self.DetectPlayerOnLadder.OnComponentBeginOverlap`
  (params (OverlappedComponent :type "PrimitiveComponent Object Reference") (OtherActor :type "Actor Object Reference") (OtherComp :type "PrimitiveComponent Object Reference") (OtherBodyIndex :type Integer) (bFromSweep :type Boolean) (SweepResult :type "HitResult Structure (by ref)"))
  (bind _asbp_third_person_character (cast `/Game/ThirdPerson/Blueprints/BP_ThirdPersonCharacter` OtherActor))
  (`/Engine/EditorBlueprintResources/StandardMacros.IsValid` _asbp_third_person_character
    (:`Is Valid`
      (set `/Game/ThirdPerson/Blueprints/BP_ThirdPersonCharacter.LadderClimbing` true _asbp_third_person_character))))

(event `self.DetectPlayerOnLadder.OnComponentEndOverlap`
  (params (OverlappedComponent :type "PrimitiveComponent Object Reference") (OtherActor :type "Actor Object Reference") (OtherComp :type "PrimitiveComponent Object Reference") (OtherBodyIndex :type Integer))
  (bind _asbp_third_person_character (cast `/Game/ThirdPerson/Blueprints/BP_ThirdPersonCharacter` OtherActor))
  (`/Engine/EditorBlueprintResources/StandardMacros.IsValid` _asbp_third_person_character
    (:`Is Valid`
      (set `/Game/ThirdPerson/Blueprints/BP_ThirdPersonCharacter.LadderClimbing` false _asbp_third_person_character)
      (set `/Game/ThirdPerson/Blueprints/BP_ThirdPersonCharacter.GetOnTheLadder` false _asbp_third_person_character)
      (`/Game/ThirdPerson/Blueprints/BP_ThirdPersonCharacter.MakeClimingFalse` _asbp_third_person_character))))

(event `self.DetectUpSide.OnComponentBeginOverlap`
  (params (OverlappedComponent :type "PrimitiveComponent Object Reference") (OtherActor :type "Actor Object Reference") (OtherComp :type "PrimitiveComponent Object Reference") (OtherBodyIndex :type Integer) (bFromSweep :type Boolean) (SweepResult :type "HitResult Structure (by ref)"))
  (bind _asbp_third_person_character (cast `/Game/ThirdPerson/Blueprints/BP_ThirdPersonCharacter` OtherActor))
  (`/Engine/EditorBlueprintResources/StandardMacros.IsValid` _asbp_third_person_character
    (:`Is Valid`
      (if (not (`/Game/ThirdPerson/Blueprints/BP_ThirdPersonCharacter.PlayerOnTopTrue` _asbp_third_person_character))
        (set `/Game/ThirdPerson/Blueprints/BP_ThirdPersonCharacter.StopInputs` true _asbp_third_person_character)
        (set `/Game/ThirdPerson/Blueprints/BP_ThirdPersonCharacter.LadderClimbing` true _asbp_third_person_character)
        (set `/Game/ThirdPerson/Blueprints/BP_ThirdPersonCharacter.EndLadderClimbing` true _asbp_third_person_character)
        (`KismetSystemLibrary.Delay` 3.2)
        (`SceneComponent.K2_SetWorldLocation` (`Character.CapsuleComponent` _asbp_third_person_character) (`SceneComponent.K2_GetComponentLocation` (`self.Arrow`)) false false)))))

(event `self.DetectUpSide.OnComponentEndOverlap`
  (params (OverlappedComponent :type "PrimitiveComponent Object Reference") (OtherActor :type "Actor Object Reference") (OtherComp :type "PrimitiveComponent Object Reference") (OtherBodyIndex :type Integer))
  (bind _asbp_third_person_character (cast `/Game/ThirdPerson/Blueprints/BP_ThirdPersonCharacter` OtherActor))
  (`/Engine/EditorBlueprintResources/StandardMacros.IsValid` _asbp_third_person_character
    (:`Is Valid`
      (set `/Game/ThirdPerson/Blueprints/BP_ThirdPersonCharacter.StopInputs` false _asbp_third_person_character)
      (set `/Game/ThirdPerson/Blueprints/BP_ThirdPersonCharacter.LadderClimbing` false _asbp_third_person_character)
      (set `/Game/ThirdPerson/Blueprints/BP_ThirdPersonCharacter.EndLadderClimbing` false _asbp_third_person_character))))

(event `self.Player OnFloor.OnComponentBeginOverlap`
  (params (OverlappedComponent :type "PrimitiveComponent Object Reference") (OtherActor :type "Actor Object Reference") (OtherComp :type "PrimitiveComponent Object Reference") (OtherBodyIndex :type Integer) (bFromSweep :type Boolean) (SweepResult :type "HitResult Structure (by ref)"))
  (bind _asbp_third_person_character (cast `/Game/ThirdPerson/Blueprints/BP_ThirdPersonCharacter` OtherActor))
  (`/Engine/EditorBlueprintResources/StandardMacros.IsValid` _asbp_third_person_character
    (:`Is Valid`
      (set `/Game/ThirdPerson/Blueprints/BP_ThirdPersonCharacter.PlayerOnGroundTrue` true _asbp_third_person_character)
      (set `/Game/ThirdPerson/Blueprints/BP_ThirdPersonCharacter.PlayerOnTopTrue` false _asbp_third_person_character))))

(event `self.Player OnFloor.OnComponentEndOverlap`
  (params (OverlappedComponent :type "PrimitiveComponent Object Reference") (OtherActor :type "Actor Object Reference") (OtherComp :type "PrimitiveComponent Object Reference") (OtherBodyIndex :type Integer))
  (bind _asbp_third_person_character (cast `/Game/ThirdPerson/Blueprints/BP_ThirdPersonCharacter` OtherActor))
  (`/Engine/EditorBlueprintResources/StandardMacros.IsValid` _asbp_third_person_character
    (:`Is Valid`
      (set `/Game/ThirdPerson/Blueprints/BP_ThirdPersonCharacter.PlayerOnGroundTrue` false _asbp_third_person_character))))

(event `self.Player On Top.OnComponentBeginOverlap`
  (params (OverlappedComponent :type "PrimitiveComponent Object Reference") (OtherActor :type "Actor Object Reference") (OtherComp :type "PrimitiveComponent Object Reference") (OtherBodyIndex :type Integer) (bFromSweep :type Boolean) (SweepResult :type "HitResult Structure (by ref)"))
  (bind _asbp_third_person_character (cast `/Game/ThirdPerson/Blueprints/BP_ThirdPersonCharacter` OtherActor))
  (`/Engine/EditorBlueprintResources/StandardMacros.IsValid` _asbp_third_person_character
    (:`Is Valid`
      (set `/Game/ThirdPerson/Blueprints/BP_ThirdPersonCharacter.PlayerOnTopTrue` true _asbp_third_person_character))))

(event `self.Player On Top.OnComponentEndOverlap`
  (params (OverlappedComponent :type "PrimitiveComponent Object Reference") (OtherActor :type "Actor Object Reference") (OtherComp :type "PrimitiveComponent Object Reference") (OtherBodyIndex :type Integer))
  (bind _asbp_third_person_character (cast `/Game/ThirdPerson/Blueprints/BP_ThirdPersonCharacter` OtherActor))
  (`/Engine/EditorBlueprintResources/StandardMacros.IsValid` _asbp_third_person_character))

(fn `UserConstructionScript`)